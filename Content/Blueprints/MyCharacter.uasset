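; Player character for what appears to be an auto-scrolling flying shooter, pushed constantly along world +X each tick.
; Axis inputs add sideways and vertical movement relative to the control rotation.
; The fire action spawns a LaserProjectile at both left and right cannons with zero rotation, then plays a laser sound at the capsule.
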(event `InputAction|FireAction`
  (params (Key :type "Key Structure"))
  (:`Pressed`
    (`|SpawnActorFromClass` "/Game/Blueprints/LaserProjectile.LaserProjectile_C" (`KismetMathLibrary.MakeTransform` (`SceneComponent.K2_GetComponentLocation` (`self.LeftCannon`))) "AdjustIfPossibleButDontSpawnIfColliding" "OverrideRootScale" null null) ; Spawn projectile
    (`|SpawnActorFromClass` "/Game/Blueprints/LaserProjectile.LaserProjectile_C" (`KismetMathLibrary.MakeTransform` (`SceneComponent.K2_GetComponentLocation` (`self.RightCannon`))) "AdjustIfPossibleButDontSpawnIfColliding" "OverrideRootScale" null null) ; Spawn projectile
    (`GameplayStatics.PlaySoundAtLocation` "/Game/Audio/LaserFire01.LaserFire01" (`SceneComponent.K2_GetComponentLocation` (`self.CapsuleComponent`)))))

(event `InputAxis|MoveLeftRight`
  (params (AxisValue :type "Float (single-precision)"))
  (`self.AddMovementInput` (`KismetMathLibrary.GetRightVector` (`self.GetControlRotation`)) AxisValue))

(event `InputAxis|MoveUpDown`
  (params (AxisValue :type "Float (single-precision)"))
  (`self.AddMovementInput` (`KismetMathLibrary.GetUpVector` (`self.GetControlRotation`)) AxisValue))

(event `self.ReceiveBeginPlay`)

(event `self.ReceiveTick`
  (params (DeltaSeconds :type "Float (single-precision)"))
  (`self.AddMovementInput` (1.0 0.0 0.0) 1.0 true))

(fn `UserConstructionScript`)